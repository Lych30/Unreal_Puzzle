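; Game mode for a tile puzzle game that starts the main menu and UI and handles new game, save, load and save deletion.
; Saving writes player position, control rotation, puzzle size and each BP_Puzzle tile's relative location to a single slot.
; Loading rebuilds the tiles at the saved size, then moves them to saved locations after a short delay and refreshes the UI.
; New game creates an initial save only when none exists.
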(event `self.ReceiveBeginPlay`
  ;[0 1 0.0959] Begin Play
  (`self.EnableInput` (`GameplayStatics.GetPlayerController` 0))
  (`KismetSystemLibrary.Delay` 0.2)
  (bind _asplayer_pawn (cast `/Game/Blueprints/Player_Pawn` (`GameplayStatics.GetPlayerPawn` 0)))
  (`/Game/Blueprints/Player_Pawn.OpenMainMenu` _asplayer_pawn)
  (bind _outactors (`GameplayStatics.GetAllActorsOfClass` "/Game/Blueprints/BP_Puzzle.BP_Puzzle_C"))
  (`/Game/UI/AC_ThomasUI.InitUI` (`self.AC_ThomasUI`) (`GameplayStatics.GetPlayerController` 0) false 0 0 (`/Game/Blueprints/BP_Puzzle.Size` (`|GetArrayItem` _outactors))))

(event `SaveGame`
  ;[0 0.07581 1] Save Game
  (bind _returnvalue (`|GenericCreateObject` "/Game/Blueprints/Saves/Save_Game.Save_Game_C"))
  (bind _asplayer_pawn (cast `/Game/Blueprints/Player_Pawn` (`GameplayStatics.GetPlayerPawn` 0)))
  (set `/Game/Blueprints/Saves/Save_Game.PlayerPosition` (`self.K2_GetActorLocation` _asplayer_pawn) _returnvalue)
  (set `/Game/Blueprints/Saves/Save_Game.PlayerRotation` (`Controller.GetControlRotation` (`GameplayStatics.GetPlayerController` 0)) _returnvalue)
  (bind _outactors (`GameplayStatics.GetAllActorsOfClass` "/Game/Blueprints/BP_Puzzle.BP_Puzzle_C"))
  (bind _output (`|GetArrayItem` _outactors))
  (set `/Game/Blueprints/Saves/Save_Game.size` (`/Game/Blueprints/BP_Puzzle.Size` _output) _returnvalue)
  (for (_array_element _array_index) (`/Game/Blueprints/BP_Puzzle.Tiles` _output)
    (bind _relativelocation (`SceneComponent.RelativeLocation` _array_element))
    (`KismetArrayLibrary.Array_Set` (`/Game/Blueprints/Saves/Save_Game.PuzzlePlanes1Rotations` _returnvalue) _array_index _relativelocation true)
    (`KismetSystemLibrary.PrintString` (`KismetStringLibrary.Conv_VectorToString` _relativelocation)))
  (`GameplayStatics.SaveGameToSlot` _returnvalue "Save1"))

(event `LoadGame`
  ;[1 1 1] Load Game
  (bind _returnvalue (`GameplayStatics.LoadGameFromSlot` "Save1"))
  (bind _assave_game (cast `/Game/Blueprints/Saves/Save_Game` _returnvalue)
    (:`then`
      (`self.K2_SetActorLocation` (`GameplayStatics.GetPlayerPawn` 0) (`/Game/Blueprints/Saves/Save_Game.PlayerPosition` _assave_game) false true)
      (`Controller.SetControlRotation` (`GameplayStatics.GetPlayerController` 0) (`/Game/Blueprints/Saves/Save_Game.PlayerRotation` _assave_game))
      (bind _outactors (`GameplayStatics.GetAllActorsOfClass` "/Game/Blueprints/BP_Puzzle.BP_Puzzle_C"))
      (bind _output (`|GetArrayItem` _outactors))
      (set `/Game/Blueprints/BP_Puzzle.Size` (`/Game/Blueprints/Saves/Save_Game.size` _assave_game) _output)
      (set `/Game/Blueprints/BP_Puzzle.Spacing` 60.0 _output)
      (`/Game/Blueprints/BP_Puzzle.PopulateTiles` _output)
      (`KismetSystemLibrary.Delay` 0.2)
      (for (_array_element _array_index) (`/Game/Blueprints/BP_Puzzle.Tiles` _output)
        (bind _puzzleplanes1rotations (`/Game/Blueprints/Saves/Save_Game.PuzzlePlanes1Rotations` _assave_game))
        (if (> (`KismetArrayLibrary.Array_Length` _puzzleplanes1rotations) _array_index)
          (`SceneComponent.K2_SetRelativeLocation` _array_element (`|GetArrayItem` _puzzleplanes1rotations _array_index) false true)))
      (bind _size (`/Game/Blueprints/BP_Puzzle.Size` _output))
      (`/Game/UI/AC_ThomasUI.InitUI` (`self.AC_ThomasUI`) (`GameplayStatics.GetPlayerController` 0) false 0 0 _size)
      (bind _foundwidgets (`WidgetBlueprintLibrary.GetAllWidgetsOfClass` "/Game/UI/UI_GameUI.UI_GameUI_C"))
      (bind _returnvalue_2 (`KismetStringLibrary.Conv_IntToString` _size))
      (`TextBlock.SetText` (`/Game/UI/UI_GameUI.TextBlock` (`|GetArrayItem` _foundwidgets)) (`KismetTextLibrary.Conv_StringToText` (`KismetStringLibrary.Concat_StrStr` _returnvalue_2 "X" _returnvalue_2))))
    (:`CastFailed`
      (`KismetSystemLibrary.PrintString` "No Save"))))

(event `NewGame`
  ;[1 1 1] New Game
  (bind _outactors (`GameplayStatics.GetAllActorsOfClass` "/Game/Blueprints/BP_Puzzle.BP_Puzzle_C"))
  (`/Game/UI/AC_ThomasUI.InitUI` (`self.AC_ThomasUI`) (`GameplayStatics.GetPlayerController` 0) false 0 0 (`/Game/Blueprints/BP_Puzzle.Size` (`|GetArrayItem` _outactors)))
  (`WidgetBlueprintLibrary.SetInputMode_GameOnly` (`GameplayStatics.GetPlayerController` 0))
  (bind _returnvalue (`GameplayStatics.DoesSaveGameExist` "Save1"))
  (if (not _returnvalue)
    (bind _returnvalue_2 (`GameplayStatics.CreateSaveGameObject` "/Game/Blueprints/Saves/Save_Game.Save_Game_C"))
    (`GameplayStatics.SaveGameToSlot` _returnvalue_2 "Save1")
    (`self.SaveGame`)
    (`KismetSystemLibrary.Delay` 0.2)
    (bind _outactors_2 (`GameplayStatics.GetAllActorsOfClass` "/Game/Blueprints/Player_Pawn.Player_Pawn_C"))
    (`/Game/Blueprints/Player_Pawn.CreateMenus` (`|GetArrayItem` _outactors_2))))

(event `InputAction|DeleteSave`
  (params (Key :type "Key Structure"))
  ;[1 1 1] DeleteSave
  (:`Pressed`
    (`GameplayStatics.DeleteGameInSlot` "Save1")))

(fn `UserConstructionScript`)