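; Blueprint for a 3x3 puzzle that rearranges nine plane components by swapping their positions.
; BeginPlay gathers the planes into PlaneArray, and Swap takes two planes as input.
; Swap prints "Too far" when they exceed a distance threshold; otherwise it caches their world locations while looping the array, then exchanges them.
; Nothing in this Blueprint calls Swap, shuffles the planes or checks for a solved state.
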(event `self.ReceiveBeginPlay`
  (set `self.PlaneArray` (`|MakeArray` (`self.Plane0`) (`self.Plane1`) (`self.Plane2`) (`self.Plane3`) (`self.Plane4`) (`self.Plane5`) (`self.Plane6`) (`self.Plane7`) (`self.Plane8`))))

(fn `Swap`
  (params (Plane1 :type "StaticMeshComponent Object Reference") (Plane2 :type "StaticMeshComponent Object Reference"))
  (if (> (`KismetMathLibrary.Vector_Distance` (`SceneComponent.K2_GetComponentLocation` Plane1) (`SceneComponent.K2_GetComponentLocation` Plane2)) 40.0)
    (`KismetSystemLibrary.PrintString` "Too far")
    (else
      (`|ExecutionSequence`
        (:`then_0`
          (for _array_element (`self.PlaneArray`)
            (if (== _array_element Plane1)
              (set `self.PlanePos1` (`SceneComponent.K2_GetComponentLocation` Plane1))
              (elif (== _array_element Plane2)
                (set `self.PlanePos2` (`SceneComponent.K2_GetComponentLocation` Plane2))))))
        (:`then_1`
          (`SceneComponent.K2_SetWorldLocation` Plane1 (`self.PlanePos2`) false false)
          (`SceneComponent.K2_SetWorldLocation` Plane1 (`self.PlanePos2`) false false)
          (`SceneComponent.K2_SetWorldLocation` Plane2 (`self.PlanePos1`) false false))))))

(fn `UserConstructionScript`)