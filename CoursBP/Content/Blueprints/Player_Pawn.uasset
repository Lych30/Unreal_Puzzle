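; First-person flying player pawn for a tile puzzle, with a crosshair, pause menu and main menu widget.
; Input flags set a movement direction each tick from control rotation, while the mouse steers the view.
; SelectTile increments the UI move counter before a camera trace asks BP_Puzzle to swap the hit tile with the empty one, so misses also count.
; TrySelectTile, a two-pick swap for 3x3_Puzzle_BP, is not called here.
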(event `self.ReceiveBeginPlay`
  ;[0 1 0.08333] BeginPlay
  (`self.EnableInput` (`GameplayStatics.GetPlayerController` 0))
  (bind _returnvalue (`|CreateWidget` "/Game/Widgets/UI_CrossHair.UI_CrossHair_C"))
  (`UserWidget.AddToViewport` _returnvalue 0)
  (`self.CreateMenus`))

(event `self.ReceiveTick`
  (params (DeltaSeconds :type "Float (single-precision)"))
  ;[1 0 0] Update
  (`self.Movements`))

(event `CreateMenus`
  (bind _returnvalue (`GameplayStatics.GetPlayerController` 0))
  ;[0 0.1887 1] Menus
  (bind _returnvalue_2 (`|CreateWidget` "/Game/Widgets/MenuWidget.MenuWidget_C" _returnvalue))
  (set `self.MainMenuWidget` _returnvalue_2)
  (bind _returnvalue_3 (`|CreateWidget` "/Game/Widgets/PauseWidget.PauseWidget_C" _returnvalue))
  (set `self.PauseMenuWidget` _returnvalue_3))

(event `InputAction|Forward` :consume false
  (params (Key :type "Key Structure"))
  ;[0.09912 0.06801 1] Inputs
  ;;[1 1 1] Actions
  (:`Pressed`
    (set `self.Forward` true))
  (:`Released`
    (set `self.Forward` false)))

(event `InputAction|Straff_Left` :consume false
  (params (Key :type "Key Structure"))
  ;[0.09912 0.06801 1] Inputs
  ;;[1 1 1] Actions
  (:`Pressed`
    (set `self.Straff_Left` true))
  (:`Released`
    (set `self.Straff_Left` false)))

(event `InputAxisKey|MouseY`
  (params (AxisValue :type "Float (single-precision)"))
  ;[0.09912 0.06801 1] Inputs
  ;;[1 1 1] Mouse
  (`self.AddControllerPitchInput` (* AxisValue -1.0)))

(event `InputAction|Backward` :consume false
  (params (Key :type "Key Structure"))
  ;[0.09912 0.06801 1] Inputs
  ;;[1 1 1] Actions
  (:`Pressed`
    (set `self.Backward` true))
  (:`Released`
    (set `self.Backward` false)))

(event `InputAxisKey|MouseX`
  (params (AxisValue :type "Float (single-precision)"))
  ;[0.09912 0.06801 1] Inputs
  ;;[1 1 1] Mouse
  (`self.AddControllerYawInput` AxisValue))

(event `InputAction|Up`
  (params (Key :type "Key Structure"))
  ;[0.09912 0.06801 1] Inputs
  ;;[1 1 1] Actions
  (:`Pressed`
    (set `self.Up` true))
  (:`Released`
    (set `self.Up` false)))

(event `InputAction|Straff_Right` :consume false
  (params (Key :type "Key Structure"))
  ;[0.09912 0.06801 1] Inputs
  ;;[1 1 1] Actions
  (:`Pressed`
    (set `self.Straff_Right` true))
  (:`Released`
    (set `self.Straff_Right` false)))

(event `InputAction|Down`
  (params (Key :type "Key Structure"))
  ;[0.09912 0.06801 1] Inputs
  ;;[1 1 1] Actions
  (:`Pressed`
    (set `self.Down` true))
  (:`Released`
    (set `self.Down` false)))

(event `InputAction|Pause`
  (params (Key :type "Key Structure"))
  ;[0.09912 0.06801 1] Inputs
  ;;[1 1 1] Actions
  (:`Pressed`
    (`self.OpenPause`)))

(event `InputAction|SelectTile`
  (params (Key :type "Key Structure"))
  ;[0.09912 0.06801 1] Inputs
  ;;[1 1 1] Actions
  (:`Pressed`
    (`self.SwapTileWithEmpty`)))

(fn `Movements`
  (bind _returnvalue (`KismetMathLibrary.GetForwardVector` (`self.GetControlRotation`)))
  (bind _returnvalue_2 (`KismetMathLibrary.GetRightVector` (`self.GetControlRotation`)))
  (set `self.Direction` (0.0 0.0 0.0))
  (if (`self.Forward`)
    (set `self.Direction` _returnvalue))
  (if (`self.Backward`)
    (set `self.Direction` (* _returnvalue -1.0)))
  (if (`self.Straff_Right`)
    (set `self.Direction` (* -1.0 _returnvalue_2)))
  (if (`self.Straff_Left`)
    (set `self.Direction` _returnvalue_2))
  (if (`self.Up`)
    (set `self.Direction` (+ (`self.Direction`) (0.0 0.0 1.0))))
  (if (`self.Down`)
    (set `self.Direction` (+ (`self.Direction`) (0.0 0.0 -1.0))))
  (`self.AddMovementInput` (`self.Direction`)))

(fn `OpenMainMenu`
  (bind _returnvalue (`GameplayStatics.GetPlayerController` 0))
  (bind _mainmenuwidget (`self.MainMenuWidget`))
  (`UserWidget.AddToViewport` _mainmenuwidget 0)
  (`WidgetBlueprintLibrary.SetInputMode_UIOnlyEx` _returnvalue _mainmenuwidget)
  (set `PlayerController.bShowMouseCursor` true _returnvalue))

(fn `OpenPause`
  (bind _returnvalue (`GameplayStatics.GetPlayerController` 0))
  (bind _pausemenuwidget (`self.PauseMenuWidget`))
  (if (`Widget.IsInViewport` _pausemenuwidget)
    (`Widget.RemoveFromParent` (`self.PauseMenuWidget`))
    (`GameplayStatics.SetGamePaused` false)
    (else
      (`UserWidget.AddToViewport` _pausemenuwidget 0)
      (`GameplayStatics.SetGamePaused` true)
      (set `PlayerController.bShowMouseCursor` true _returnvalue)
      (`WidgetBlueprintLibrary.SetInputMode_UIOnlyEx` _returnvalue _pausemenuwidget))))

(fn `SwapTileWithEmpty`
  (bind _returnvalue (`SceneComponent.K2_GetComponentLocation` (`self.Camera`)))
  (bind _foundwidgets (`WidgetBlueprintLibrary.GetAllWidgetsOfClass` "/Game/UI/UI_GameUI.UI_GameUI_C"))
  (`/Game/UI/UI_GameUI.UI_IncreamentMovement` (`|GetArrayItem` _foundwidgets))
  (bind _outhit (`KismetSystemLibrary.LineTraceSingle` _returnvalue (+ _returnvalue (* (`KismetMathLibrary.GetForwardVector` (`self.GetControlRotation`)) 1000.0)) "TraceTypeQuery1"))
  (bind (_bblockinghit _binitialoverlap _time _distance _location _impactpoint _normal _impactnormal _physmat _hitactor _hitcomponent) (`GameplayStatics.BreakHitResult` _outhit))
  (bind _asbp_puzzle (cast `/Game/Blueprints/BP_Puzzle` _hitactor))
  (bind _astile_component (cast `/Game/Blueprints/TileComponent` _hitcomponent))
  (`/Game/Blueprints/BP_Puzzle.SwapWithEmpty` _asbp_puzzle _astile_component))

(fn `TrySelectTile`
  (bind _returnvalue (`SceneComponent.K2_GetComponentLocation` (`self.Camera`)))
  (bind _outhit (`KismetSystemLibrary.LineTraceSingle` _returnvalue (+ _returnvalue (* (`KismetMathLibrary.GetForwardVector` (`self.GetControlRotation`)) 1000.0)) "TraceTypeQuery1"))
  (if (`KismetStringLibrary.Contains` (`KismetSystemLibrary.GetObjectName` (`.HitComponent` (`GameplayStatics.BreakHitResult` _outhit))) "Plane")
    (bind (_bblockinghit _binitialoverlap _time _distance _location _impactpoint _normal _impactnormal _physmat _hitactor _hitcomponent) (`GameplayStatics.BreakHitResult` _outhit))
    (bind _asstatic_mesh_component (cast `StaticMeshComponent` _hitcomponent))
    (if (`KismetSystemLibrary.IsValid` (`self.Plane1`))
      (bind _output_get (set `self.Plane2` _asstatic_mesh_component))
      (`KismetSystemLibrary.PrintString` (`KismetSystemLibrary.GetDisplayName` _output_get))
      (bind _as3x_3_puzzle_bp (cast `/Game/Blueprints/3x3_Puzzle_BP` _hitactor))
      (`/Game/Blueprints/3x3_Puzzle_BP.Swap` _as3x_3_puzzle_bp (stale _output_get_2) _output_get)
      (set `self.Plane1` null)
      (set `self.Plane2` null)
      (else
        (bind _output_get_2 (set `self.Plane1` _asstatic_mesh_component))
        (`KismetSystemLibrary.PrintString` (`KismetSystemLibrary.GetDisplayName` _output_get_2))))))

(fn `UserConstructionScript`)