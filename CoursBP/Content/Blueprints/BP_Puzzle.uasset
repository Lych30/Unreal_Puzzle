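; BP_Puzzle is a sliding-tile picture puzzle board, with its functions invoked externally as the event graph is empty.
; PopulateTiles rebuilds a Size×Size grid of tile components, slices one material across them via per-tile tiling/offset instances, empties the last tile and updates the UI size label.
; SwapWithEmpty swaps a nearby axis-aligned tile with the empty one.
; ShuffleTiles randomly permutes all positions without checking solvability.
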(event `self.ReceiveBeginPlay`)

(fn `DeleteAllTiles`
  (bind _tiles (`self.Tiles`))
  (`KismetSystemLibrary.PrintString` "Delete all")
  (for _array_element _tiles
    (`ActorComponent.K2_DestroyComponent` _array_element))
  (`KismetArrayLibrary.Array_Clear` _tiles)
  (set `self.TileIndex` 0)
  (set `self.EmptyTile` null))

(fn `PopulateTiles`
  (bind _size (`self.Size`))
  (bind _spacing (`self.Spacing`))
  (bind _tiles (`self.Tiles`))
  (bind _returnvalue (`KismetStringLibrary.Conv_IntToString` (`self.Size`)))
  (bind _returnvalue_2 (/ 1 (`self.Size`)))
  (bind _returnvalue_3 (`KismetStringLibrary.Concat_StrStr` _returnvalue "X" _returnvalue))
  (bind _output (`|GetArrayItem` _tiles (`KismetArrayLibrary.Array_LastIndex` _tiles)))
  (if (not (`KismetArrayLibrary.Array_IsEmpty` (`self.Tiles`)))
    (`self.DeleteAllTiles`))
  (for _index (range 1 (+ _size 1))
    (for _index_2 (range 1 (+ _size 1))
      (bind _result (`/Engine/EditorBlueprintResources/StandardMacros.IncrementInt` (`self.TileIndex`))
        (:`  `
          (set `self.TileIndex` _result)
          (bind _returnvalue_4 (`KismetMathLibrary.MakeVector` (* _index _spacing) (* (* _index_2 _spacing) -1.0)))
          (bind _returnvalue_5 (`|AddComponentByClass` "/Game/Blueprints/TileComponent.TileComponent_C" false (`KismetMathLibrary.MakeTransform` _returnvalue_4 (struct) (0.5 0.5 0.5))))
          (set `/Game/Blueprints/TileComponent.BasePosition` _returnvalue_4 _returnvalue_5)
          (`KismetArrayLibrary.Array_Add` (`self.Tiles`) _returnvalue_5)
          (bind _returnvalue_6 (`KismetMaterialLibrary.CreateDynamicMaterialInstance` "/Game/Materials/Materials/TilingAndOffset_Mat.TilingAndOffset_Mat"))
          (`MaterialInstanceDynamic.SetScalarParameterValue` _returnvalue_6 "U Tiling" _returnvalue_2)
          (`MaterialInstanceDynamic.SetScalarParameterValue` _returnvalue_6 "V Tiling" _returnvalue_2)
          (`MaterialInstanceDynamic.SetScalarParameterValue` _returnvalue_6 "U Offset" (/ _index (`self.Size`)))
          (`MaterialInstanceDynamic.SetScalarParameterValue` _returnvalue_6 "V Offset" (/ _index_2 (`self.Size`)))
          (`PrimitiveComponent.SetMaterial` _returnvalue_5 0 _returnvalue_6)))))
  ;[1 1 1] Set last one as the empty one
  (`/Game/Blueprints/TileComponent.SetEmpty` _output)
  (set `self.EmptyTile` _output)
  ;[1 1 1] Setup UI Size
  (bind _foundwidgets (`WidgetBlueprintLibrary.GetAllWidgetsOfClass` "/Game/UI/UI_GameUI.UI_GameUI_C"))
  (`TextBlock.SetText` (`/Game/UI/UI_GameUI.TextBlock` (`|GetArrayItem` _foundwidgets)) (`KismetTextLibrary.Conv_StringToText` _returnvalue_3))
  (`KismetSystemLibrary.PrintString` _returnvalue_3))

(fn `ShuffleTiles`
  (bind _templocs (`self.TempLocs`))
  (for _array_element (`self.Tiles`)
    (`KismetArrayLibrary.Array_Add` _templocs (`SceneComponent.RelativeLocation` _array_element)))
  (`KismetArrayLibrary.Array_Shuffle` _templocs)
  (for (_array_element_2 _array_index) _templocs
    (`SceneComponent.K2_SetRelativeLocation` (`|GetArrayItem` (`self.Tiles`) _array_index) _array_element_2 false false)))

(fn `SwapWithEmpty`
  (params (TargetTile :type "/Game/Blueprints/TileComponent Object Reference"))
  (bind _emptytile (`self.EmptyTile`))
  (bind _relativelocation (`SceneComponent.RelativeLocation` TargetTile))
  (bind (_x _y) (`KismetMathLibrary.BreakVector3f` _relativelocation))
  (bind _relativelocation_2 (`SceneComponent.RelativeLocation` (`self.EmptyTile`)))
  (bind (_x_2 _y_2) (`KismetMathLibrary.BreakVector3f` _relativelocation_2))
  (if (and (<= (`KismetMathLibrary.Vector_Distance2D` _relativelocation _relativelocation_2) (+ (`self.Spacing`) 50.0)) (or (== _x _x_2) (== _y _y_2)))
    ;[1 1 1] Swap locations
    (bind _output_get (set `self.TempLoc` (`SceneComponent.GetRelativeTransform` TargetTile)))
    (`SceneComponent.K2_SetRelativeTransform` TargetTile (`SceneComponent.GetRelativeTransform` _emptytile) false true)
    (`SceneComponent.K2_SetRelativeTransform` _emptytile _output_get false true)))

(fn `UserConstructionScript`)