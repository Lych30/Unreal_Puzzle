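; BP_FirstActor is a test actor that swaps two string variables when the left mouse button is released.
; On BeginPlay it enables input from the first player controller.
; Each release prints StringA and StringB, exchanges their values through a temporary string, then prints both again to show the result.
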(event `self.ReceiveBeginPlay`
  (`self.EnableInput` (`GameplayStatics.GetPlayerController` 0)))

(event `Key|LeftMouseButton` :paused true
  (params (Key :type "Key Structure"))
  (:`Released`
    (`KismetSystemLibrary.PrintString` (`self.StringA`))
    (`KismetSystemLibrary.PrintString` (`self.StringB`))
    (set `self.TempString` (`self.StringA`))
    (set `self.StringA` (`self.StringB`))
    (set `self.StringB` (`self.TempString`))
    (`KismetSystemLibrary.PrintString` (`self.StringA`))
    (`KismetSystemLibrary.PrintString` (`self.StringB`))))

(fn `UserConstructionScript`)