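; BP_Puzzle is a sliding-tile puzzle actor built from a square grid of tile components, with the last one empty.
; PopulateTiles spawns tiles storing their home positions and ShuffleTiles randomly permutes their locations, though neither call is wired to an event.
; SwapWithEmpty swaps axis-aligned neighbors with the empty tile, then calls CheckForVictory.
; CheckForVictory compares tiles to home positions, but prints "Victory!" even after breaking on a mismatch.
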(event `self.ReceiveBeginPlay`)

(fn `CheckForVictory`
  (for _array_element (`self.Tiles`)
    (if (not (== (`SceneComponent.RelativeLocation` _array_element) (`/Game/Game_Blueprints/TileComponent.BasePosition` _array_element) :`ErrorTolerance` 2.0))
      (break)))
  (`KismetSystemLibrary.PrintString` "Victory!"))

(fn `DeleteAllTiles`
  (for _array_element (`self.K2_GetComponentsByClass` "/Game/Game_Blueprints/TileComponent.TileComponent_C")
    (`ActorComponent.K2_DestroyComponent` _array_element)))

(fn `PopulateTiles`
  (bind _size (`self.Size`))
  (bind _spacing (`self.Spacing`))
  (bind _tiles (`self.Tiles`))
  (bind _output (`|GetArrayItem` _tiles (`KismetArrayLibrary.Array_LastIndex` _tiles)))
  (for _index (range 1 (+ _size 1))
    (for _index_2 (range 1 (+ _size 1))
      (bind _result (`/Engine/EditorBlueprintResources/StandardMacros.IncrementInt` (`self.TileIndex`))
        (:`  `
          (set `self.TileIndex` _result)
          (bind _returnvalue (`KismetMathLibrary.MakeVector` (* _index _spacing) (* (* _index_2 _spacing) -1.0)))
          (bind _returnvalue_2 (`|AddComponentByClass` "/Game/Game_Blueprints/TileComponent.TileComponent_C" false (`KismetMathLibrary.MakeTransform` _returnvalue (struct) (0.5 0.5 0.5))))
          (set `/Game/Game_Blueprints/TileComponent.BasePosition` _returnvalue _returnvalue_2)
          (`KismetArrayLibrary.Array_Add` (`self.Tiles`) _returnvalue_2)))))
  ;[1 1 1] Set last one as the empty one
  (`/Game/Game_Blueprints/TileComponent.SetEmpty` _output)
  (set `self.EmptyTile` _output))

(fn `ShuffleTiles`
  (bind _templocs (`self.TempLocs`))
  (for _array_element (`self.Tiles`)
    (`KismetArrayLibrary.Array_Add` _templocs (`SceneComponent.RelativeLocation` _array_element)))
  (`KismetArrayLibrary.Array_Shuffle` _templocs)
  (for (_array_element_2 _array_index) _templocs
    (`SceneComponent.K2_SetRelativeLocation` (`|GetArrayItem` (`self.Tiles`) _array_index) _array_element_2 false false)))

(fn `SwapWithEmpty`
  (params (TargetTile :type "/Game/Game_Blueprints/TileComponent Object Reference"))
  (bind _emptytile (`self.EmptyTile`))
  (bind _relativelocation (`SceneComponent.RelativeLocation` TargetTile))
  (bind (_x _y) (`KismetMathLibrary.BreakVector3f` _relativelocation))
  (bind _relativelocation_2 (`SceneComponent.RelativeLocation` (`self.EmptyTile`)))
  (bind (_x_2 _y_2) (`KismetMathLibrary.BreakVector3f` _relativelocation_2))
  (if (and (<= (`KismetMathLibrary.Vector_Distance2D` _relativelocation _relativelocation_2) (+ (`self.Spacing`) 50.0)) (or (== _x _x_2) (== _y _y_2)))
    ;[1 1 1] Swap locations
    (bind _output_get (set `self.TempLoc` (`SceneComponent.GetRelativeTransform` TargetTile)))
    (`SceneComponent.K2_SetRelativeTransform` TargetTile (`SceneComponent.GetRelativeTransform` _emptytile) false true)
    (`SceneComponent.K2_SetRelativeTransform` _emptytile _output_get false true)
    (`self.CheckForVictory`)))

(fn `UserConstructionScript`)